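; MovingLogObstacle_BP is a moving obstacle that hovers on four hover components and shuttles between two points.
; A looping timer, set to the timeline's length, flip-flops the target and restarts the movement timeline with a distance-based play rate.
; Each update lerps X and Y from the current location for a slowing approach, leaving Z untouched and zeroing roll to prevent rolling.
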(event Custom|MoveObstacleToTarget
  (bind _obstaclemesh (Variables|Default|GetObstacleMesh))
  (bind _relativerotation (Variables|/Script/Engine.SceneComponent|GetRelativeRotation _obstaclemesh))
  ;[1 1 1] Swaps between target points each time the event is called
  (Utilities|FlowControl|FlipFlop
    (:A
      (Variables|Default|SetTargetPoint (Variables|Default|GetPoint1)))
    (:B
      (Variables|Default|SetTargetPoint (Variables|Default|GetPoint2))))
  ;[1 1 1] Moves obstacle between points
  (Components|Timeline|SetPlayRate (Variables|Default|GetMovementTimeline) (/ (Math|Vector|VectorLength (- (Transformation|GetWorldLocation (Variables|Default|GetObstacleMesh)) (Transformation|GetWorldLocation (Variables|Default|GetTargetPoint)))) 3e+04))
  (bind _movementtrack (Timeline|MovementTimeline PlayFromStart)
    (:Update
      (Transformation|SetWorldLocation (Variables|Default|GetObstacleMesh) (Math|Vector|MakeVector (.X (Math|Vector|BreakVector (Math|Vector|Lerp(Vector) (Transformation|GetWorldLocation (Variables|Default|GetObstacleMesh)) (Transformation|GetWorldLocation (Variables|Default|GetTargetPoint)) _movementtrack))) (.Y (Math|Vector|BreakVector (Math|Vector|Lerp(Vector) (Transformation|GetWorldLocation (Variables|Default|GetObstacleMesh)) (Transformation|GetWorldLocation (Variables|Default|GetTargetPoint)) _movementtrack))) (.z (Transformation|GetWorldLocation (Variables|Default|GetObstacleMesh)))) false false)
      ;[1 1 1] Prevents object from rolling
      (Transformation|SetRelativeRotation _obstaclemesh (Math|Rotator|MakeRotator 0.0 (.pitch _relativerotation) (.yaw _relativerotation)) false false))))

(event EventBeginPlay
  (Default|InitComponent (Variables|Default|GetHoverComponent_SC) (Variables|Default|GetObstacleMesh))
  (Default|InitComponent (Variables|Default|GetHoverComponent_SC1) (Variables|Default|GetObstacleMesh))
  (Default|InitComponent (Variables|Default|GetHoverComponent_SC2) (Variables|Default|GetObstacleMesh))
  (Default|InitComponent (Variables|Default|GetHoverComponent_SC3) (Variables|Default|GetObstacleMesh))
  (Utilities|Time|SetTimerbyEvent (delegate Custom|MoveObstacleToTarget) (Components|Timeline|GetTimelineLength (Variables|Default|GetMovementTimeline)) true))

(fn ConstructionScript)