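; Checkpoint manager that tracks each player's boat progress through a race's checkpoints.
; Init binds to the hit event of the supplied checkpoints and caches the Finish_BP actor.
; Hits update the boat's current checkpoint only in sequence and broadcast CheckpointUpdated, except that the last checkpoint on lap 3 skips the order check, enables finishing and shows the finish plane.
; The GameStateChanged handler switches on state but does nothing.
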(event Custom|CheckpointHit
  (params (Checkpoint%20Number :type Integer) (Player :type Integer))
  ;[1 1 1] Checkpoint Hit
  (bind _asbase_boat_pawn (Utilities|Casting|CastToBaseBoat_Pawn (Pawn|GetControlledPawn (Class|GameplayStatics|GetPlayerControllerfromID Player))))
  (if (== (Variables|/Game/Migrate/Blueprints/BoatPawns/BaseBoat_Pawn.BaseBoat_Pawn_C|GetCurrentLap _asbase_boat_pawn) 3)
    (if (== (- Checkpoint%20Number 1) (Utilities|Array|LastIndex (Variables|Default|GetCheckpoints)))
      (Variables|/Game/Migrate/Blueprints/BoatPawns/BaseBoat_Pawn.BaseBoat_Pawn_C|SetcanEnd? _asbase_boat_pawn true)
      (Rendering|SetVisibility (Variables|/Game/Migrate/Blueprints/Finish_BP.Finish_BP_C|GetPlane (Variables|Default|GetFinish)) true false)
      (Variables|/Game/Migrate/Blueprints/BoatPawns/BaseBoat_Pawn.BaseBoat_Pawn_C|SetCurrentCheckpoint _asbase_boat_pawn Checkpoint%20Number :!label _label)
      (Default|CallCheckpointUpdated Player)
      (else
        (if (== Checkpoint%20Number (+ (Variables|/Game/Migrate/Blueprints/BoatPawns/BaseBoat_Pawn.BaseBoat_Pawn_C|GetCurrentCheckpoint _asbase_boat_pawn) 1)) :!label _label_2
          (goto _label))))
    (else
      (goto _label_2))))

(event Custom|Init
  (params (Checkpoints :type Array%20of%20Checkpoint%20Object%20References))
  ;[1 1 1] Init
  (bind _output_get (Variables|Default|SetCheckpoints Checkpoints))
  (EventDispatchers|BindEventtoCheckpointHit _output_get (EventDispatchers|CreateEvent :!event Custom|CheckpointHit))
  (bind _returnvalue (Actor|GetActorOfClass "/Game/Migrate/Blueprints/Finish_BP.Finish_BP_C"))
  (Variables|Default|SetFinish _returnvalue))

(event EventGameStateChanged
  (params (newGameState :type E_GameState%20Enum :default "NewEnumerator0"))
  ;[1 1 1] GameStateChanged
  (switch Utilities|FlowControl|Switch|SwitchonE_GameState newGameState))

(fn ConstructionScript)