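; Race manager for a two-player boat race that tracks each player's checkpoint and lap progress and refreshes their race UI.
; Init binds to checkpoint, checkpoint-update and finish-line events, whose handlers record progress in per-player maps or go straight to the UI update.
; CheckPositions picks the leader by lap, then checkpoint, but its result is unused: the UI always receives Winning as false.
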(event Custom|Init
  (params (Checkpoints :type Array%20of%20Checkpoint%20Object%20References))
  ;[1 1 1] Init
  (EventDispatchers|BindEventtoCheckpointHit Checkpoints (EventDispatchers|CreateEvent :!event Custom|CheckpointHit))
  (bind _returnvalue (Actor|GetActorOfClass "/Game/Migrate/Blueprints/Managers/Checkpoint_Manager.Checkpoint_Manager_C"))
  (EventDispatchers|BindEventtoCheckpointUpdated _returnvalue (EventDispatchers|CreateEvent :!event Custom|CheckpointUpdated))
  (bind _returnvalue_2 (Actor|GetActorOfClass "/Game/Migrate/Blueprints/Finish_BP.Finish_BP_C"))
  (EventDispatchers|BindEventtoFinishLine _returnvalue_2 (EventDispatchers|CreateEvent :!event Custom|FinishLine)))

(event Custom|CheckpointHit
  (params (Checkpoint%20Number :type Integer) (Player :type Integer))
  ;[1 1 1] CheckpointHit
  (Utilities|Map|Add (Variables|Default|GetPlayerCheckpointPositions) (+ Player 1) Checkpoint%20Number)
  ;[1 1 1] CheckpointUpdated
  (bind _winning_player (CallFunction|CheckPositions))
  (bind _asgm_race (Utilities|Casting|CastToGM_Race (Game|GetGameMode)))
  (bind _asbase_boat_pawn (Utilities|Casting|CastToBaseBoat_Pawn (Pawn|GetControlledPawn (Class|GameplayStatics|GetPlayerControllerfromID Player))))
  (Default|UpdateUI (Utilities|Array|Get(acopy) (Variables|/Game/Migrate/Blueprints/GameModes/GM_Race.GM_Race_C|GetRace%20UI _asgm_race) Player) (Variables|/Game/Migrate/Blueprints/BoatPawns/BaseBoat_Pawn.BaseBoat_Pawn_C|GetCurrentCheckpoint _asbase_boat_pawn) (Variables|/Game/Migrate/Blueprints/BoatPawns/BaseBoat_Pawn.BaseBoat_Pawn_C|GetCurrentLap _asbase_boat_pawn) false))

(event Custom|CheckpointUpdated
  (params (Player :type Integer))
  ;[1 1 1] CheckpointUpdated
  (bind _asgm_race (Utilities|Casting|CastToGM_Race (Game|GetGameMode)))
  (bind _asbase_boat_pawn (Utilities|Casting|CastToBaseBoat_Pawn (Pawn|GetControlledPawn (Class|GameplayStatics|GetPlayerControllerfromID (stale Custom|CheckpointHit Player)))))
  (Default|UpdateUI (Utilities|Array|Get(acopy) (Variables|/Game/Migrate/Blueprints/GameModes/GM_Race.GM_Race_C|GetRace%20UI _asgm_race) (stale Custom|CheckpointHit Player)) (Variables|/Game/Migrate/Blueprints/BoatPawns/BaseBoat_Pawn.BaseBoat_Pawn_C|GetCurrentCheckpoint _asbase_boat_pawn) (Variables|/Game/Migrate/Blueprints/BoatPawns/BaseBoat_Pawn.BaseBoat_Pawn_C|GetCurrentLap _asbase_boat_pawn) false))

(event Custom|FinishLine
  (params (Player :type Integer) (NewParam :type Integer))
  (Utilities|Map|Add (Variables|Default|GetPlayerLapPositions) (+ Player 1) NewParam)
  ;[1 1 1] CheckpointUpdated
  (bind _winning_player (CallFunction|CheckPositions))
  (bind _asgm_race (Utilities|Casting|CastToGM_Race (Game|GetGameMode)))
  (bind _asbase_boat_pawn (Utilities|Casting|CastToBaseBoat_Pawn (Pawn|GetControlledPawn (Class|GameplayStatics|GetPlayerControllerfromID (stale Custom|CheckpointHit Player)))))
  (Default|UpdateUI (Utilities|Array|Get(acopy) (Variables|/Game/Migrate/Blueprints/GameModes/GM_Race.GM_Race_C|GetRace%20UI _asgm_race) (stale Custom|CheckpointHit Player)) (Variables|/Game/Migrate/Blueprints/BoatPawns/BaseBoat_Pawn.BaseBoat_Pawn_C|GetCurrentCheckpoint _asbase_boat_pawn) (Variables|/Game/Migrate/Blueprints/BoatPawns/BaseBoat_Pawn.BaseBoat_Pawn_C|GetCurrentLap _asbase_boat_pawn) false))

(fn ConstructionScript)

(fn CheckPositions
  (bind _playerlappositions (Variables|Default|GetPlayerLapPositions))
  (bind _playercheckpointpositions (Variables|Default|GetPlayerCheckpointPositions))
  (bind _value (Utilities|Map|Find _playerlappositions 1))
  (bind _value_2 (Utilities|Map|Find _playerlappositions 2))
  (if (== _value _value_2)
    (if (> (.Value (Utilities|Map|Find _playercheckpointpositions 1)) (.Value (Utilities|Map|Find _playercheckpointpositions 2)))
      _
      (else
        (return 1)))
    (elif (> _value _value_2)
      _
      (else
        (return 1))))
  (return 0))