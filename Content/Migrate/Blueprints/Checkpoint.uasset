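; Checkpoint actor for boat races that reports when a player's boat passes it in the correct order.
; When a player-controlled boat leaves the Box trigger, it checks that its CheckpointNumber is one above the boat's CurrentCheckpoint.
; On a match it fires the CheckpointHit dispatcher with the checkpoint number and player controller ID, leaving progress updates to listeners.
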(event OnComponentEndOverlap(Box)
  (params (OverlappedComponent :type Primitive%20Component%20Object%20Reference) (OtherActor :type Actor%20Object%20Reference) (OtherComp :type Primitive%20Component%20Object%20Reference) (OtherBodyIndex :type Integer))
  (bind _asbase_boat_pawn (Utilities|Casting|CastToBaseBoat_Pawn OtherActor))
  (bind _asboat_pc (Utilities|Casting|CastToBoat_PC (Pawn|GetController _asbase_boat_pawn)))
  (if (== (+ (Variables|/Game/Migrate/Blueprints/BoatPawns/BaseBoat_Pawn.BaseBoat_Pawn_C|GetCurrentCheckpoint _asbase_boat_pawn) 1) (Variables|Default|GetCheckpointNumber))
    (Default|CallCheckpointHit (Variables|Default|GetCheckpointNumber) (Class|GameplayStatics|GetPlayerControllerID _asboat_pc))))

(fn ConstructionScript)