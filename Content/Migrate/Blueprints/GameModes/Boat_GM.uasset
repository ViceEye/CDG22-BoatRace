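; Boat_GM is a game mode Blueprint for a boat level that manages the map UI and pause flow.
; BeginPlay adds the map widget to the viewport after a short delay.
; Pause shows a pause menu and pauses the game, or opens the MainMenu level if already paused, while Resume removes the menu and unpauses.
; The construction script caches all BoatSpawner actors in an array, which this file never reads.
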(event Custom|Pause
  (if (Game|IsGamePaused)
    (Game|OpenLevel(byName) "MainMenu")
    (else
      (bind _returnvalue (UserInterface|CreateWidget "/Game/EdwardsFile/UI/PauseMenu.PauseMenu_C"))
      (bind _output_get (Variables|Default|SetPauseMenu _returnvalue))
      (UserInterface|Viewport|AddtoViewport _output_get 0)
      (Game|SetGamePaused true))))

(event Custom|Resume
  (if (Game|IsGamePaused)
    (Widget|RemovefromParent (Variables|Default|GetPauseMenu))
    (Game|SetGamePaused false)))

(event EventBeginPlay
  (Utilities|FlowControl|Delay 0.2)
  (bind _returnvalue (UserInterface|CreateWidget (Variables|Default|GetWidgetClass)))
  (bind _output_get (Variables|Default|SetMapUI _returnvalue))
  (UserInterface|Viewport|AddtoViewport _output_get 0))

(fn ConstructionScript
  (bind _outactors (Actor|GetAllActorsOfClass "/Game/Migrate/Blueprints/BoatSpawner.BoatSpawner_C"))
  (Variables|Default|SetBoatSpawnerArray _outactors))