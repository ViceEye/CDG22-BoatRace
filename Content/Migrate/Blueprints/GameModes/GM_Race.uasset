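; Game mode for a local split-screen boat race, handling player setup, match flow and pausing.
; A state machine runs Setup, PreGame, InGame and PostGame, broadcasting changes to I_GameState actors and widgets.
; It creates local players, spawns their selected boats at BoatSpawners, and starts checkpoint, race, ultimate and two per-player points managers.
; InGame adds checkpoint counters; Finish_BP's RuleComplete event leads unconditionally to the end screen.
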(event Custom|Pause
  (bind _returnvalue (Game|GetPlayerController 0))
  ;[1 1 1] Pause
  (Game|SetGamePaused true)
  (bind _returnvalue_2 (UserInterface|CreateWidget "/Game/EdwardsFile/EdwardsFileUpdate/UI/PauseMenu_Final.PauseMenu_Final_C"))
  (Variables|Default|SetPauseMenu_New _returnvalue_2)
  (UserInterface|Viewport|AddtoViewport (Variables|Default|GetPauseMenu_New) 0)
  (Input|SetInputModeUIOnly _returnvalue 0 "DoNotLock")
  (Variables|/Script/Engine.PlayerController|SetbShowMouseCursor _returnvalue true))

(event Custom|Init
  ;[1 1 1] Init
  (Class|GameplayStatics|SetForceDisableSplitscreen false)
  (bind _ascustom_boat_game_instance (Utilities|Casting|CastToCustomBoatGameInstance (Game|GetGameInstance)))
  (Variables|Default|SetGameInstanceRef _ascustom_boat_game_instance)
  (Input|SetInputModeGameOnly (Game|GetPlayerController 0))
  (CallFunction|RemoveOtherPlayers)
  (CallFunction|ChangeGameState "NewEnumerator0"))

(event Custom|RuleComplete
  (params (WinningPlayer :type Integer))
  ;[1 1 1] Check Rule
  (Variables|Default|SetisRuleComplete? true)
  (CallFunction|CanEndCheck))

(event Custom|Setup
  (bind _self self)
  (bind _optionsstring (Variables|Default|GetOptionsString _self))
  (bind _returnvalue (Class|GameplayStatics|GetIntOption _optionsstring "playerCount" 2))
  ;[1 1 1] Setup
  (Utilities|FlowControl|Delay 0.2)
  (CallFunction|SetUpControllers _returnvalue)
  (Variables|Default|SetPlayerCount _returnvalue)
  (CallFunction|ChangeGameState "NewEnumerator1"))

(event Custom|Pregame
  ;[1 1 1] Pregame
  (Utilities|FlowControl|Delay 0.2)
  (CallFunction|SpawnCharacters)
  (CallFunction|GetCheckpoints)
  (bind _returnvalue (Game|SpawnActorfromClass "/Game/Migrate/Blueprints/Managers/Checkpoint_Manager.Checkpoint_Manager_C" (Math|Transform|MakeTransform "0, 0, 0" "0, 0, 0" "1,1,1") "Undefined" 0 0))
  (bind _output_get (Variables|Default|SetCheckpointManager _returnvalue))
  (Default|Init _output_get (Variables|Default|GetCheckpoints))
  (bind _returnvalue_2 (Game|SpawnActorfromClass "/Game/Migrate/Blueprints/Managers/NewRace_Manager.NewRace_Manager_C" (Math|Transform|MakeTransform "0, 0, 0" "0, 0, 0" "1,1,1") "Undefined" 0 0))
  (bind _output_get_2 (Variables|Default|SetRaceManager _returnvalue_2))
  (Default|Init _output_get_2 (Variables|Default|GetCheckpoints))
  (bind _returnvalue_3 (Game|SpawnActorfromClass "/Game/Migrate/Blueprints/UltimateComponents/UltimateManager.UltimateManager_C" (Math|Transform|MakeTransform "0, 0, 0" "0, 0, 0" "1,1,1") "Undefined" 0 0))
  (Variables|Default|SetUltimateManager _returnvalue_3)
  (bind _returnvalue_4 (Game|SpawnActorfromClass "/Game/Migrate/Blueprints/KanevPointsSystem/PointsManager.PointsManager_C" (Math|Transform|MakeTransform "0, 0, 0" "0, 0, 0" "1,1,1") "Undefined" 0 0))
  (bind _output_get_3 (Variables|Default|SetP1PointsManager _returnvalue_4))
  (Default|InitP1 _output_get_3)
  (bind _returnvalue_5 (Game|SpawnActorfromClass "/Game/Migrate/Blueprints/KanevPointsSystem/PointsManagerPlayer2.PointsManagerPlayer2_C" (Math|Transform|MakeTransform "0, 0, 0" "0, 0, 0" "1,1,1") "Undefined" 0 0))
  (bind _output_get_4 (Variables|Default|SetPointsManager2 _returnvalue_5))
  (Default|InitP2 _output_get_4)
  (CallFunction|ChangeGameState "NewEnumerator2"))

(event Custom|Resume
  (bind _returnvalue (Game|GetPlayerController 0))
  ;[1 1 1] Resume
  (Game|SetGamePaused false)
  (Widget|RemovefromParent (Variables|Default|GetPauseMenu_New))
  (Input|SetInputModeGameOnly _returnvalue)
  (Variables|/Script/Engine.PlayerController|SetbShowMouseCursor _returnvalue false))

(event Custom|In%20Game
  ;[1 1 1] InGame
  (for _array_element (Variables|Default|GetPlayerControllers)
    (bind _returnvalue (UserInterface|CreateWidget "/Game/UI/CheckpointCounter_UI.CheckpointCounter_UI_C" _array_element))
    (Utilities|Array|AddUnique (Variables|Default|GetRace%20UI) _returnvalue)
    (UserInterface|Viewport|AddtoPlayerScreen _returnvalue)))

(event Custom|Post%20Game
  (bind _returnvalue (Game|GetPlayerController 0))
  ;[1 1 1] Post Game
  (bind _returnvalue_2 (UserInterface|CreateWidget "/Game/UI/EndScreen.EndScreen_C"))
  (UserInterface|Viewport|AddtoViewport _returnvalue_2 0)
  (Default|UpdateUI _returnvalue_2 (stale Custom|RuleComplete WinningPlayer))
  (Input|SetInputModeUIOnly _returnvalue 0 "DoNotLock")
  (Variables|/Script/Engine.PlayerController|SetbShowMouseCursor _returnvalue true))

(event EventBeginPlay
  ;[1 1 1] Begin
  (CallFunction|Init))

(event EventPostLogin
  (params (NewPlayer :type Player%20Controller%20Object%20Reference))
  ;[1 1 1] Add and Remove Controllers
  (Utilities|Array|Add (Variables|Default|GetPlayerControllers) NewPlayer))

(event EventOnLogout
  (params (ExitingController :type Controller%20Object%20Reference))
  ;[1 1 1] Add and Remove Controllers
  (bind _asplayer_controller (Utilities|Casting|CastToPlayerController ExitingController))
  (Utilities|Array|RemoveItem (Variables|Default|GetPlayerControllers) _asplayer_controller))

(fn ConstructionScript)

(fn SetUpControllers
  (params (Number%20of%20Players :type Integer))
  (bind _result (Math|Integer|DecrementInt Number%20of%20Players)
    (:%20%20
      (for _index (range 0 _result)
        (bind _returnvalue (Class|GameplayStatics|CreatePlayer _index))))))

(fn RemoveOtherPlayers
  (for _index (range 0 3)
    (Utilities|IsValid (Class|GameplayStatics|GetPlayerControllerfromID _index)
      (:Is%20Valid
        (Class|GameplayStatics|RemovePlayer (Class|GameplayStatics|GetPlayerControllerfromID _index) true)))))

(fn ChangeGameState
  (params (NewGameState :type E_GameState%20Enum :default "NewEnumerator0"))
  (Variables|Default|SetcurrentGameState NewGameState)
  (bind _outactors (Actor|GetAllActorswithInterface "/Game/Migrate/Blueprints/I_GameState.I_GameState_C"))
  (for _array_element _outactors
    (Class|IGameState|GameStateChanged(Message) _array_element NewGameState))
  (bind _foundwidgets (Class|WidgetBlueprintLibrary|GetAllWidgetswithInterface "/Game/Migrate/Blueprints/I_GameState.I_GameState_C" false))
  (for _array_element_2 _foundwidgets
    (Class|IGameState|GameStateChanged(Message) _array_element_2 NewGameState))
  (switch Utilities|FlowControl|Switch|SwitchonE_GameState NewGameState
    (:NewEnumerator0
      (CallFunction|Setup))
    (:NewEnumerator1
      (CallFunction|Pregame))
    (:NewEnumerator2
      (CallFunction|InGame))
    (:NewEnumerator3
      (CallFunction|PostGame))))

(fn SpawnCharacters
  (for _array_element (Variables|Default|GetPlayerControllers)
    (CallFunction|SpawnPawn _array_element)))

(fn SpawnPawn
  (params (Player%20Controller :type Player%20Controller%20Object%20Reference))
  (bind _playercontrollers (Variables|Default|GetPlayerControllers))
  (bind _returnvalue (Utilities|Array|FindItem _playercontrollers Player%20Controller))
  (bind _spawnertransform (CallFunction|GetSpawners _returnvalue))
  (bind _returnvalue_2 (Game|SpawnActorfromClass (Utilities|Array|Get(acopy) (Variables|/Game/Migrate/Blueprints/CustomBoatGameInstance.CustomBoatGameInstance_C|GetPlayerSelections (Variables|Default|GetGameInstanceRef)) _returnvalue) (Math|Transform|MakeTransform (.location _spawnertransform) (.rotation _spawnertransform) "1,1,1") "AdjustIfPossibleButAlwaysSpawn" 0 0))
  (Pawn|Possess Player%20Controller _returnvalue_2))

(fn GetSpawners
  (params (ControllerIndex :type Integer))
  (bind _outactors (Actor|GetAllActorsOfClass "/Game/Migrate/Blueprints/BoatSpawner.BoatSpawner_C"))
  (for (_array_element _array_index) _outactors
    (if (== _array_index ControllerIndex)
      (LocalVariables|SettempSpawner _array_element)))
  (return (Math|Transform|MakeTransform (Transformation|GetActorLocation (LocalVariables|GettempSpawner)) (Transformation|GetActorRotation (LocalVariables|GettempSpawner)) "1,1,1")))

(fn CanEndCheck
  (if true
    (CallFunction|ChangeGameState "NewEnumerator3")
    (return true)
    (else
      (return false))))

(fn GetCheckpoints
  (bind _outactors (Actor|GetAllActorsOfClass "/Game/Migrate/Blueprints/Checkpoint.Checkpoint_C"))
  (Variables|Default|SetCheckpoints _outactors)
  (bind _returnvalue (Actor|GetActorOfClass "/Game/Migrate/Blueprints/Finish_BP.Finish_BP_C"))
  (EventDispatchers|BindEventtoRuleComplete _returnvalue (EventDispatchers|CreateEvent :!event Custom|RuleComplete)))