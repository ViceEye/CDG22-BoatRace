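; Finish line actor for a boat race that counts laps and ends the race.
; On BeginPlay it gathers all Checkpoint actors, and a boat overlapping the box after the last checkpoint gains a lap, resets its checkpoint and fires FinishLine.
; Reaching lap three reveals a plane mesh.
; A boat with CanEnd instead fires FinishLine and RuleComplete with its player number, then disables the box collision so only the first finisher counts.
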(event OnComponentBeginOverlap(Box)
  (params (OverlappedComponent :type Primitive%20Component%20Object%20Reference) (OtherActor :type Actor%20Object%20Reference) (OtherComp :type Primitive%20Component%20Object%20Reference) (OtherBodyIndex :type Integer) (bFromSweep :type Boolean) (SweepResult :type Hit%20Result%20Structure%20%28by%20ref%29))
  ;[1 1 1] BeginOverlap
  (bind _asbase_boat_pawn (Utilities|Casting|CastToBaseBoat_Pawn OtherActor))
  (if (Variables|/Game/Migrate/Blueprints/BoatPawns/BaseBoat_Pawn.BaseBoat_Pawn_C|GetcanEnd? _asbase_boat_pawn)
    (bind _asboat_pc (Utilities|Casting|CastToBoat_PC (Pawn|GetController _asbase_boat_pawn)))
    (Default|CallFinishLine)
    (Default|CallRuleComplete (+ (Class|GameplayStatics|GetPlayerControllerID _asboat_pc) 1))
    (Collision|SetCollisionEnabled (Variables|Default|GetBox) "NoCollision")
    (else
      (bind _asboat_pc_2 (Utilities|Casting|CastToBoat_PC (Pawn|GetController _asbase_boat_pawn)))
      (if (== (Utilities|Array|LastIndex (Variables|Default|GetCheckpoints)) (- (Variables|/Game/Migrate/Blueprints/BoatPawns/BaseBoat_Pawn.BaseBoat_Pawn_C|GetCurrentCheckpoint _asbase_boat_pawn) 1))
        (bind _output_get (Variables|/Game/Migrate/Blueprints/BoatPawns/BaseBoat_Pawn.BaseBoat_Pawn_C|SetCurrentLap _asbase_boat_pawn (+ (Variables|/Game/Migrate/Blueprints/BoatPawns/BaseBoat_Pawn.BaseBoat_Pawn_C|GetCurrentLap _asbase_boat_pawn) 1)))
        (Variables|/Game/Migrate/Blueprints/BoatPawns/BaseBoat_Pawn.BaseBoat_Pawn_C|SetCurrentCheckpoint _asbase_boat_pawn 0)
        (Default|CallFinishLine (Class|GameplayStatics|GetPlayerControllerID _asboat_pc_2) _output_get)
        (if (== (Variables|/Game/Migrate/Blueprints/BoatPawns/BaseBoat_Pawn.BaseBoat_Pawn_C|GetCurrentLap _asbase_boat_pawn) 3)
          (Rendering|SetVisibility (Variables|Default|GetPlane) true false))))))

(event Custom|Init
  ;[1 1 1] Init
  (bind _outactors (Actor|GetAllActorsOfClass "/Game/Migrate/Blueprints/Checkpoint.Checkpoint_C"))
  (Variables|Default|SetCheckpoints _outactors))

(event EventBeginPlay
  (CallFunction|Init))

(fn ConstructionScript)