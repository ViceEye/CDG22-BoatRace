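; UltimateManager runs the boat players' ultimate abilities: Bath, EggSplat, MuddyWater, Raccoon and TeaTime.
; Each calls UltimateAbilityUsed, then Bath alters the user's speed and turning, while others hit every other player with screen splats, slowdown, flipped camera or disabled movement.
; Timer events revert effects through references from the last loop pass, so only the last target is restored.
; ResetTeaTime re-enables the Detector but leaves CanMove false.
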(event Custom|Bath
  (params (Controller :type Player%20Controller%20Object%20Reference) (Speed :type Float%20%28single-precision%29) (Turn :type Float%20%28single-precision%29) (Duration :type Float%20%28single-precision%29))
  ;[1 1 1] Bath
  (Utilities|FlowControl|Sequence
    (:then_0
      (Default|CallUltimateAbilityUsed self))
    (:then_1
      (bind _asbase_boat_pawn (Utilities|Casting|CastToBaseBoat_Pawn (Pawn|GetControlledPawn Controller)))
      (Variables|/Game/Migrate/Blueprints/BoatPawns/BaseBoat_Pawn.BaseBoat_Pawn_C|SetForwardSpeed _asbase_boat_pawn (+ (Variables|/Game/Migrate/Blueprints/BoatPawns/BaseBoat_Pawn.BaseBoat_Pawn_C|GetForwardSpeed _asbase_boat_pawn) Speed))
      (Variables|/Game/Migrate/Blueprints/BoatPawns/BaseBoat_Pawn.BaseBoat_Pawn_C|SetTurningSpeed _asbase_boat_pawn (- (Variables|/Game/Migrate/Blueprints/BoatPawns/BaseBoat_Pawn.BaseBoat_Pawn_C|GetTurningSpeed _asbase_boat_pawn) Turn))
      (Utilities|Time|SetTimerbyEvent (delegate Custom|ResetBath) Duration))))

(event Custom|Remove%20Widget
  ;[1 1 1] Egg Splat
  (Widget|RemovefromParent (stale Custom|EggSplat _returnvalue)))

(event Custom|EggSplat
  (params (Controller :type Player%20Controller%20Object%20Reference) (PlayerControllers :type Array%20of%20Player%20Controller%20Object%20References) (Duration :type Float%20%28single-precision%29))
  ;[1 1 1] Egg Splat
  (Utilities|FlowControl|Sequence
    (:then_0
      (Default|CallUltimateAbilityUsed self))
    (:then_1
      (for _array_element PlayerControllers
        (if (not (== Controller _array_element))
          (bind _returnvalue (UserInterface|CreateWidget "/Game/UI/EggSplatUI.EggSplatUI_C" _array_element))
          (UserInterface|Viewport|AddtoPlayerScreen _returnvalue)
          (Utilities|Time|SetTimerbyEvent (delegate Custom|Remove%20Widget) Duration))))))

(event Custom|ResetBath
  ;[1 1 1] Bath
  (Variables|/Game/Migrate/Blueprints/BoatPawns/BaseBoat_Pawn.BaseBoat_Pawn_C|SetForwardSpeed (stale Custom|Bath _asbase_boat_pawn) (- (Variables|/Game/Migrate/Blueprints/BoatPawns/BaseBoat_Pawn.BaseBoat_Pawn_C|GetForwardSpeed (stale Custom|Bath _asbase_boat_pawn)) (stale Custom|Bath Speed)))
  (Variables|/Game/Migrate/Blueprints/BoatPawns/BaseBoat_Pawn.BaseBoat_Pawn_C|SetTurningSpeed (stale Custom|Bath _asbase_boat_pawn) (+ (Variables|/Game/Migrate/Blueprints/BoatPawns/BaseBoat_Pawn.BaseBoat_Pawn_C|GetTurningSpeed (stale Custom|Bath _asbase_boat_pawn)) (stale Custom|Bath Turn))))

(event Custom|TeaTime
  (params (Controller :type Player%20Controller%20Object%20Reference) (PlayerControllers :type Array%20of%20Player%20Controller%20Object%20References) (Duration :type Float%20%28single-precision%29))
  ;[1 1 1] Teacup
  (Utilities|FlowControl|Sequence
    (:then_0
      (Default|CallUltimateAbilityUsed self))
    (:then_1
      (for _array_element PlayerControllers
        (if (not (== Controller _array_element))
          (bind _asbase_boat_pawn (Utilities|Casting|CastToBaseBoat_Pawn (Pawn|GetControlledPawn _array_element)))
          (Variables|/Game/Migrate/Blueprints/Detector.Detector_C|SetEnable (Variables|/Game/Migrate/Blueprints/BoatPawns/BaseBoat_Pawn.BaseBoat_Pawn_C|GetDetector _asbase_boat_pawn) false)
          (Variables|/Game/Migrate/Blueprints/BoatPawns/BaseBoat_Pawn.BaseBoat_Pawn_C|SetcanMove _asbase_boat_pawn false)
          (Utilities|Time|SetTimerbyEvent (delegate Custom|ResetTeaTime) Duration))))))

(event Custom|ResetMuddy
  ;[1 1 1] Muddy Water
  (Variables|/Game/Migrate/Blueprints/BoatPawns/BaseBoat_Pawn.BaseBoat_Pawn_C|SetForwardSpeed (stale Custom|MuddyWater _asbase_boat_pawn) (+ (Variables|/Game/Migrate/Blueprints/BoatPawns/BaseBoat_Pawn.BaseBoat_Pawn_C|GetForwardSpeed (stale Custom|MuddyWater _asbase_boat_pawn)) (stale Custom|MuddyWater Amount))))

(event Custom|MuddyWater
  (params (Controller :type Player%20Controller%20Object%20Reference) (PlayerControllers :type Array%20of%20Player%20Controller%20Object%20References) (Amount :type Float%20%28single-precision%29) (Duration :type Float%20%28single-precision%29))
  ;[1 1 1] Muddy Water
  (Utilities|FlowControl|Sequence
    (:then_0
      (Default|CallUltimateAbilityUsed self))
    (:then_1
      (for _array_element PlayerControllers
        (if (not (== Controller _array_element))
          (bind _asbase_boat_pawn (Utilities|Casting|CastToBaseBoat_Pawn (Pawn|GetControlledPawn _array_element)))
          (Variables|/Game/Migrate/Blueprints/BoatPawns/BaseBoat_Pawn.BaseBoat_Pawn_C|SetForwardSpeed _asbase_boat_pawn (- (Variables|/Game/Migrate/Blueprints/BoatPawns/BaseBoat_Pawn.BaseBoat_Pawn_C|GetForwardSpeed _asbase_boat_pawn) Amount))
          (Utilities|Time|SetTimerbyEvent (delegate Custom|ResetMuddy) Duration))))))

(event Custom|ResetTeaTime
  ;[1 1 1] Teacup
  (Variables|/Game/Migrate/Blueprints/Detector.Detector_C|SetEnable (Variables|/Game/Migrate/Blueprints/BoatPawns/BaseBoat_Pawn.BaseBoat_Pawn_C|GetDetector (stale Custom|TeaTime _asbase_boat_pawn)) true))

(event Custom|Raccoon
  (params (Controller :type Player%20Controller%20Object%20Reference) (PlayerControllers :type Array%20of%20Player%20Controller%20Object%20References) (Duration :type Float%20%28single-precision%29))
  ;[1 1 1] Raccoon
  (Utilities|FlowControl|Sequence
    (:then_0
      (Default|CallUltimateAbilityUsed self))
    (:then_1
      (for _array_element PlayerControllers
        (if (not (== Controller _array_element))
          (bind _asbase_boat_pawn (Utilities|Casting|CastToBaseBoat_Pawn (Pawn|GetControlledPawn _array_element)))
          (Variables|/Game/Migrate/Blueprints/BoatPawns/BaseBoat_Pawn.BaseBoat_Pawn_C|SetCanUseCameraFlip _asbase_boat_pawn false)
          (Transformation|SetRelativeRotation (Variables|/Game/Migrate/Blueprints/BoatPawns/BaseBoat_Pawn.BaseBoat_Pawn_C|GetSpringArm _asbase_boat_pawn) "0,180.000000, 0" false false)
          (Utilities|Time|SetTimerbyEvent (delegate Custom|ResetRaccoon) Duration))))))

(event Custom|ResetRaccoon
  ;[1 1 1] Raccoon
  (Variables|/Game/Migrate/Blueprints/BoatPawns/BaseBoat_Pawn.BaseBoat_Pawn_C|SetCanUseCameraFlip (stale Custom|Raccoon _asbase_boat_pawn) true)
  (Transformation|SetRelativeRotation (Variables|/Game/Migrate/Blueprints/BoatPawns/BaseBoat_Pawn.BaseBoat_Pawn_C|GetSpringArm (stale Custom|Raccoon _asbase_boat_pawn)) "0, 0, 0" false false))

(fn ConstructionScript)