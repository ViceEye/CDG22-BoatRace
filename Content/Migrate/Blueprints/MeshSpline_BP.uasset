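; MeshSpline_BP is a construction-time tool actor that builds spline mesh segments along its MeshSpline.
; The construction script derives section length from the actor's Y scale, then loops over the spline's length in those steps.
; Each step adds two spline mesh components sharing X forward axis, local start/end positions and tangents clamped to section length to follow the curve.
; The event graph holds no active logic.
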(event EventBeginPlay)

(event Collision|EventActorBeginOverlap
  (params (OtherActor :type Actor%20Object%20Reference)))

(event EventTick
  (params (DeltaSeconds :type Float%20%28single-precision%29)))

(fn ConstructionScript
  (bind _mesh_spline (Variables|Default|GetMesh_Spline))
  (bind _mesh_spline_2 (Variables|Default|GetMesh_Spline))
  (Variables|Default|SetSection_Lenght (* (.y (Transformation|GetActorScale3D)) 199.0))
  (for _index (range 0 (Math|Float|Truncate (/ (Spline|GetSplineLength (Variables|Default|GetMesh_Spline)) (Variables|Default|GetSection_Lenght))))
    (bind _returnvalue (AddComponent|AddSplineMeshComponent false))
    (bind _returnvalue_2 (AddComponent|AddSplineMeshComponent false))
    (SplineMesh|SetForwardAxis _returnvalue_2 "X" true)
    (SplineMesh|SetStartandEnd _returnvalue_2 (Spline|GetLocationatDistanceAlongSpline _mesh_spline_2 (* _index (Variables|Default|GetSection_Lenght)) "Local") (Math|Vector|ClampVectorSize (Spline|GetTangentatDistanceAlongSpline _mesh_spline_2 (* _index (Variables|Default|GetSection_Lenght)) "Local") 0.0 (Variables|Default|GetSection_Lenght)) (Spline|GetLocationatDistanceAlongSpline _mesh_spline (* (+ _index 1) (Variables|Default|GetSection_Lenght)) "Local") (Math|Vector|ClampVectorSize (Spline|GetTangentatDistanceAlongSpline _mesh_spline (* (+ _index 1) (Variables|Default|GetSection_Lenght)) "Local") 0.0 (Variables|Default|GetSection_Lenght)) true :!class /Script/Engine.SplineMeshComponent)))