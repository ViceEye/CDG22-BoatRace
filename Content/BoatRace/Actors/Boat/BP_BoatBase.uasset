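; Base Blueprint for a boat in the boat race game, with buoyancy from four pontoons passed to a C++ setup function at construction.
; On BeginPlay it caches the BoatController and GM_Base game mode.
; Its Blueprint movement is disconnected, leaving both input axis events empty.
; That unused logic applies speed-capped acceleration forces, yaws the boat when turning with a forward nudge against spinning, and prints debug values through the controller.
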(event EventBeginPlay
  (|CallParentFunction)
  (CallFunction|RegisterController)
  (CallFunction|RegisterGamemode))

(event Collision|EventActorBeginOverlap
  (params (OtherActor :type Actor%20Object%20Reference))
  (|CallParentFunction 0))

(event EventTick
  (params (DeltaSeconds :type Float%20%28single-precision%29))
  (|CallParentFunction DeltaSeconds))

(event Input|AxisEvents|InputAxisMoveRight
  (params (AxisValue :type Float%20%28single-precision%29))
  ;[1 1 1] Blueprint-Movement
)

(event Input|AxisEvents|InputAxisMoveForward
  (params (AxisValue :type Float%20%28single-precision%29))
  ;[1 1 1] Blueprint-Movement
)

(fn ConstructionScript
  (|CallParentFunction)
  (Class|CppBoatBase|ConstructBoatBuoyancy (Utilities|Array|MakeArray (Variables|Default|GetPontoon1) (Variables|Default|GetPontoon2) (Variables|Default|GetPontoon3) (Variables|Default|GetPontoon4))) ; Set up the pontoon component within the buoyancy component via cpp so doesn't need to configure it one by one
)

(fn Popup
  (params (String :type String) (InFloat :type Float%20%28single-precision%29) (Num :type Integer))
  (Default|SetPopupInfo (Variables|/Game/BoatRace/Blueprints/BoatController.BoatController_C|GetPopupInfo (Variables|Default|GetSelfController)) (Utilities|String|Append String (Utilities|String|ToString(Float) InFloat)) Num))

(fn RegisterController
  (bind _asboat_controller (Utilities|Casting|CastToBoatController (Pawn|GetController)))
  (Variables|Default|SetSelfController _asboat_controller))

(fn RegisterGamemode
  (bind _asgm_base (Utilities|Casting|CastToGM_Base (Game|GetGameMode)))
  (Variables|Default|SetSelfGamemode _asgm_base))